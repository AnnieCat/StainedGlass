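; Directional arrow control that activates by mouse hover dwell, calling LeftArrow or RightArrow on a Buttons reference according to its Direction.
; Each tick, it line-traces the deprojected cursor against its Trigger and plays the ColorBuild timeline while hit.
; The timeline tints a dynamic material and the matching NeoPixel color on Buttons, then fires the action once on completion.
; Losing hover re-arms it, greys both NeoPixel colors and sets the timeline time.
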(event `self.ReceiveActorBeginOverlap`
  (params (OtherActor :type "Actor Object Reference")))

(event `self.ReceiveTick`
  (params (DeltaSeconds :type "Float (single-precision)"))
  (bind _linearcolor (make `LinearColor` 0.31 0.31 0.31))
  (bind _buttons (`self.Buttons`))
  (bind (_worldlocation _worlddirection) (`PlayerController.DeprojectMousePositionToWorld` (`GameplayStatics.GetPlayerController` 0)))
  (bind (_hitlocation _hitnormal _bonename _returnvalue) (`PrimitiveComponent.K2_LineTraceComponent` (`self.Trigger`) _worldlocation (+ _worldlocation (* _worlddirection 10000.0)) true false))
  (if _returnvalue
    (bind (_direction _color) (`Timeline|colorBuild` :!label _label)
      (:`Update`
        ;[1 1 1] if Interrupted
        (`MaterialInstanceDynamic.SetVectorParameterValue` (`self.dynamicMat`) "ArrowColor" _color)
        (if (`KismetStringLibrary.EqualEqual_StrStr` (`self.direction`) "LEFT")
          (set `/Game/LocalAssets/Buttons/Buttons_Bp.NeoPixel_leftArrow` _color (`self.Buttons`))
          (elif (`KismetStringLibrary.EqualEqual_StrStr` (`self.direction`) "RIGHT")
            (set `/Game/LocalAssets/Buttons/Buttons_Bp.NeoPixel_rightArrow` _color (`self.Buttons`)))))
      (:`Finished`
        (if (`KismetStringLibrary.EqualEqual_StrStr` (`self.direction`) "LEFT")
          (if (== (`self.readyToChange`) true)
            (set `self.readyToChange` false)
            (`/Game/LocalAssets/Buttons/Buttons_Bp.LeftArrow` (`self.Buttons`)))
          (elif (`KismetStringLibrary.EqualEqual_StrStr` (`self.direction`) "RIGHT")
            (if (== (`self.readyToChange`) true)
              (set `self.readyToChange` false)
              (`/Game/LocalAssets/Buttons/Buttons_Bp.RightArrow` (`self.Buttons`)))))))
    (else
      (set `self.readyToChange` true)
      (set `/Game/LocalAssets/Buttons/Buttons_Bp.NeoPixel_leftArrow` _linearcolor _buttons)
      (set `/Game/LocalAssets/Buttons/Buttons_Bp.NeoPixel_rightArrow` _linearcolor _buttons)
      (goto _label :!via `SetNewTime`))))

(fn `UserConstructionScript`
  (bind _returnvalue (`PrimitiveComponent.CreateDynamicMaterialInstance` (`self.Trigger`) 0 "/Game/LocalAssets/Arrows/SourceArrow.SourceArrow"))
  (set `self.dynamicMat` _returnvalue))