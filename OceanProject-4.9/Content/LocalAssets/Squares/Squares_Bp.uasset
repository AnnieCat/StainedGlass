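; Squares Blueprint is a paintable set of 24 square components whose windowColor changes under the mouse cursor.
; The construction script gives each square a dynamic material instance, stored by index.
; Every Tick deprojects the cursor and line-traces each component individually, applying ActiveColor to hit squares while mouseClick's Touching value is true.
; SetActiveColor changes the paint color, and resetColor recolors every square at once.
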(event `SetActiveColor`
  (params (newColor :type "Vector Structure"))
  (set `self.ActiveColor` newColor))

(event `resetColor`
  (params (resetColor :type "LinearColor Structure"))
  (for _array_element (`self.dynamic materials`)
    (`MaterialInstanceDynamic.SetVectorParameterValue` _array_element "windowColor" resetColor)))

(event `self.ReceiveTick`
  (params (DeltaSeconds :type "Float (single-precision)"))
  (bind (_worldlocation _worlddirection) (`PlayerController.DeprojectMousePositionToWorld` (`GameplayStatics.GetPlayerController` 0)))
  (for (_array_element _array_index) (`self.Get Squares Array`)
    (bind (_hitlocation _hitnormal _bonename _returnvalue) (`PrimitiveComponent.K2_LineTraceComponent` _array_element _worldlocation (+ _worldlocation (* _worlddirection 10000.0)) true false))
    (if _returnvalue
      (if (stale `mouseClick` Touching)
        (`MaterialInstanceDynamic.SetVectorParameterValue` (`KismetArrayLibrary.Array_Get` (`self.dynamic materials`) _array_index) "windowColor" (`KismetMathLibrary.Conv_VectorToLinearColor` (`self.ActiveColor`)))))))

(event `mouseClick`
  (params (Touching :type Boolean)))

(fn `Get Squares Array`
  (returns (Array :type "Array of StaticMeshComponent Object Reference"))
  (return (`|MakeArray` (`self.squares_001`) (`self.squares_002`) (`self.squares_003`) (`self.squares_004`) (`self.squares_005`) (`self.squares_006`) (`self.squares_007`) (`self.squares_008`) (`self.squares_009`) (`self.squares_010`) (`self.squares_011`) (`self.squares_012`) (`self.squares_013`) (`self.squares_014`) (`self.squares_015`) (`self.squares_016`) (`self.squares_017`) (`self.squares_018`) (`self.squares_019`) (`self.squares_020`) (`self.squares_021`) (`self.squares_022`) (`self.squares_023`) (`self.squares_024`))))

(fn `UserConstructionScript`
  (for _array_element (`self.Get Squares Array`)
    (bind _returnvalue (`PrimitiveComponent.CreateDynamicMaterialInstance` _array_element 0 null))
    (`KismetArrayLibrary.Array_Append` (`self.dynamic materials`) (`|MakeArray` _returnvalue))))