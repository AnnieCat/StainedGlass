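; GUI_Bp is an actor holding a GUI component that swings open while the mouse cursor hovers over it.
; Each tick it deprojects the cursor into a long ray and line-traces it against only its own Collider component.
; When the hover state changes, tracked by Active and LastActive, it plays the GUI_open or GUI_close timeline to drive the GUI's relative pitch.
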(event `self.ReceiveBeginPlay`)

(event `self.ReceiveTick`
  (params (DeltaSeconds :type "Float (single-precision)"))
  (bind (_worldlocation _worlddirection) (`PlayerController.DeprojectMousePositionToWorld` (`GameplayStatics.GetPlayerController` 0)))
  (bind (_hitlocation _hitnormal _bonename _returnvalue) (`PrimitiveComponent.K2_LineTraceComponent` (`self.collider`) _worldlocation (+ _worldlocation (* _worlddirection 10000.0)) true false))
  (if _returnvalue
    (set `self.active` true)
    (if (not (== (`self.active`) (`self.lastActive`)))
      (set `self.lastActive` (`self.active`))
      (bind (_direction _degrees) (`Timeline|GUI_open` :!via `PlayFromStart`)
        (:`Update`
          (`SceneComponent.K2_SetRelativeRotation` (`self.GUI`) (`KismetMathLibrary.MakeRotator` 0.0 _degrees) false false))))
    (else
      (set `self.active` false)
      (if (not (== (`self.active`) (`self.lastActive`)))
        (set `self.lastActive` (`self.active`))
        (bind (_direction_2 _degrees_2) (`Timeline|GUI_close` :!via `PlayFromStart`)
          (:`Update`
            (`SceneComponent.K2_SetRelativeRotation` (`self.GUI`) (`KismetMathLibrary.MakeRotator` 0.0 _degrees_2) false false)))))))

(event `self.ReceiveActorBeginOverlap`
  (params (OtherActor :type "Actor Object Reference")))

(fn `UserConstructionScript`)